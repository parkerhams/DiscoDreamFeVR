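; BP_PintSpawner is an actor that builds a grid of BP_PintCube actors when play begins, starting at its root's world location.
; An inner loop chains cubes along a row, placing each at the previous cube's LeftLocation, while a DoOnce captures the very first cube's FrontLocation.
; After each row a cube spawns at Front to seed the next row, and Redraw calls itself until Count exceeds Column.
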(event `Redraw`
  (for _ (range (+ (`self.Row`) 1)) :!label _label
    (bind _returnvalue (`|SpawnActorFromClass` "/Game/Import/PintableEffect/BP_PintCube.BP_PintCube_C" (`KismetMathLibrary.MakeTransform` (`self.Next`) (struct) (`self.Scale`)) "Undefined" "OverrideRootScale" null null))
    (set `self.Next` (`/Game/Import/PintableEffect/BP_PintCube.Left_Location` _returnvalue))
    (`/Engine/EditorBlueprintResources/StandardMacros.DoOnce` false
      (:`Completed`
        (set `self.Front` (`/Game/Import/PintableEffect/BP_PintCube.Front_Location` _returnvalue)))))
  (bind _returnvalue_2 (`|SpawnActorFromClass` "/Game/Import/PintableEffect/BP_PintCube.BP_PintCube_C" (`KismetMathLibrary.MakeTransform` (`self.Front`) (struct) (`self.Scale`)) "Undefined" "OverrideRootScale" null null))
  (set `self.Next` (`/Game/Import/PintableEffect/BP_PintCube.Left_Location` _returnvalue_2))
  (set `self.Front` (`/Game/Import/PintableEffect/BP_PintCube.Front_Location` _returnvalue_2))
  (if (<= (`self.Count`) (`self.Column`))
    (set `self.Count` (+ (`self.Count`) 1))
    (`self.Redraw`)))

(event `self.ReceiveBeginPlay`
  (set `self.Next` (`SceneComponent.K2_GetComponentLocation` (`self.DefaultSceneRoot`)))
  (goto _label))

(fn `UserConstructionScript`)