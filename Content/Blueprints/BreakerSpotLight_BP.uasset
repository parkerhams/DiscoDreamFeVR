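; Spot light actor that switches on once its linked breaker has been activated.
; Each tick it polls the referenced breaker's activation flag while the light is hidden, then calls TurnLightOn to toggle the spot light's visibility.
; It has no path to switch the light back off.
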(event `self.ReceiveTick`
  (params (DeltaSeconds :type "Float (single-precision)"))
  (if (and (`/Game/Blueprints/Breaker_Blueprint.HasBeenActivated` (`self.BreakerBP`)) (not (`SceneComponent.IsVisible` (`self.SpotLight`))))
    (`self.TurnLightOn`)))

(fn `TurnLightOn`
  (`SceneComponent.ToggleVisibility` (`self.SpotLight`) true))

(fn `UserConstructionScript`)