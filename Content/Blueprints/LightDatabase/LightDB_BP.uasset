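; LightDB_BP is a light switching Blueprint that toggles groups of tagged actors in the level.
; On BeginPlay it hides the root component of every actor carrying LightTag, so that group starts off.
; ActivateLights reveals that group and then hides actors carrying OffTag, swapping one set for the other.
; Visibility changes apply only to root components and do not propagate to children.
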(event `self.ReceiveBeginPlay`
  (bind _outactors (`GameplayStatics.GetAllActorsWithTag` (`self.LightTag`)))
  (for _array_element _outactors
    (`SceneComponent.SetVisibility` (`Actor.RootComponent` _array_element) false false)))

(fn `ActivateLights`
  (bind _outactors (`GameplayStatics.GetAllActorsWithTag` (`self.LightTag`)))
  (for _array_element _outactors
    (`SceneComponent.SetVisibility` (`Actor.RootComponent` _array_element) true false))
  (bind _outactors_2 (`GameplayStatics.GetAllActorsWithTag` (`self.OffTag`)))
  (for _array_element_2 _outactors_2
    (`SceneComponent.SetVisibility` (`Actor.RootComponent` _array_element_2) false false)))

(fn `UserConstructionScript`)