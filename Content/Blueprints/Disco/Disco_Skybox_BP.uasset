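; Disco skybox Blueprint that applies a sky material to its static mesh and drives a shared disco color.
; The construction script assigns the material to the mesh's first slot.
; Each tick scales the hue read from DiscoDBReference by ColorShiftSpeed and wraps it by repeated subtraction.
; The resulting fully saturated, full-brightness color is written to the Color parameter of the Disco_MPC Material Parameter Collection.
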(event `self.ReceiveTick`
  (params (DeltaSeconds :type "Float (single-precision)"))
  ;[1 1 1] Get hue, multiply it by speed modifier, and set local hue
  (bind _output_get (set `self.Local_Hue` (* (`/Game/Blueprints/Disco/Disco_DB.H` (`self.Disco_DB_Reference`)) (`self.Color_Shift_Speed`))))
  ;[1 1 1] Ensure that hue remains within range
  (while (> _output_get 359.0)
    (set `self.Local_Hue` (- _output_get 359.0)))
  ;[1 1 1] Assemble the color and set it in the Parameter Collection
  (`KismetMaterialLibrary.SetVectorParameterValue` "/Game/Blueprints/Disco/Disco_MPC.Disco_MPC" "Color" (`KismetMathLibrary.HSVToRGB` (`self.Local_Hue`) 1.0 1.0)))

(fn `UserConstructionScript`
  (`PrimitiveComponent.SetMaterial` (`self.StaticMesh`) 0 (`self.Sky_Material`)))