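; A single keypad key that shows its value and reports to its Console when interacted with.
; The construction script creates a dynamic material on the cube, writes KeyValue to the text render and sets the key to Inactive.
; Interaction passes the key itself to the Console's CheckKey.
; ChangeState stores the key state and tints the material white, green or red for inactive, valid or invalid.
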(event `/Game/Blueprints/IInteractive_BPI.InteractWithObject`
  (bind _askeypad_key_bp (cast `/Game/Blueprints/Keypad/KeypadKey_BP` self))
  (`/Game/Blueprints/Keypad/KeypadConsole_BP.CheckKey` (`self.Console`) _askeypad_key_bp))

(fn `ChangeState`
  (params (NewState :type "/Game/Blueprints/Keypad/Enum_KeyState Enum" :default "NewEnumerator0"))
  (bind _keymaterial (`self.KeyMaterial`))
  (switch `/Game/Blueprints/Keypad/Enum_KeyState` NewState ; Change material color based on KeyState
    (:`NewEnumerator0`
      ;[1 1 1] Set white if inactive
      (`MaterialInstanceDynamic.SetVectorParameterValue` _keymaterial "Color" (`KismetMathLibrary.MakeColor` 1.0 1.0 1.0)))
    (:`NewEnumerator1`
      ;[1 1 1] Set green if valid
      (`MaterialInstanceDynamic.SetVectorParameterValue` _keymaterial "Color" (`KismetMathLibrary.MakeColor` 0.0 1.0)))
    (:`NewEnumerator2`
      ;[1 1 1] Set red if invalid
      (`MaterialInstanceDynamic.SetVectorParameterValue` _keymaterial "Color" (`KismetMathLibrary.MakeColor` 1.0))))
  (set `self.KeyState` NewState))

(fn `UserConstructionScript`
  (bind _cube (`self.Cube`))
  (bind _returnvalue (`PrimitiveComponent.CreateDynamicMaterialInstance` _cube 0 (`PrimitiveComponent.GetMaterial` _cube 0) "None"))
  (set `self.KeyMaterial` _returnvalue)
  (`TextRenderComponent.K2_SetText` (`self.TextRender`) (`KismetTextLibrary.Conv_StringToText` (`self.KeyValue`)))
  (`self.ChangeState` "NewEnumerator0"))