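; KeypadConsole_BP is a keypad console Blueprint that checks entered keys against a required code.
; CheckKey appends the key's value to the submitted code, displays it and compares it character by character, clearing the entry on any mismatch.
; Matching the final character sets CodeSolved, leaving a marked spot for follow-up logic.
; Key feedback uses state enums, applied to the pressed key or to all keys through SetAllKeys.
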(fn `CheckKey`
  (params (PressedKey :type "/Game/Blueprints/Keypad/KeypadKey_BP Object Reference (by ref)"))
  (bind _returnvalue (`KismetStringLibrary.GetCharacterArrayFromString` (`self.RequiredCode`)))
  (bind _output_get (set `self.SubmittedCode` (`KismetStringLibrary.Concat_StrStr` (`self.SubmittedCode`) (`/Game/Blueprints/Keypad/KeypadKey_BP.KeyValue` PressedKey))))
  (`TextRenderComponent.K2_SetText` (`self.TextRender`) (`KismetTextLibrary.Conv_StringToText` _output_get))
  (for (_array_element _array_index) (`KismetStringLibrary.GetCharacterArrayFromString` _output_get)
    (if (`KismetStringLibrary.EqualEqual_StrStr` _array_element (`|GetArrayItem` _returnvalue _array_index))
      (if (== (`KismetArrayLibrary.Array_LastIndex` _returnvalue) _array_index)
        (`/Game/Blueprints/Keypad/KeypadKey_BP.ChangeState` PressedKey "NewEnumerator1")
        (set `self.CodeSolved` true))
      (else
        (set `self.SubmittedCode` "")
        (`/Game/Blueprints/Keypad/KeypadKey_BP.ChangeState` PressedKey "NewEnumerator2"))))
  (if (`KismetStringLibrary.NotEqual_StrStr` (`self.SubmittedCode`))
    (`/Game/Blueprints/Keypad/KeypadKey_BP.ChangeState` PressedKey "NewEnumerator2")
    (if (`self.CodeSolved`)
      (`self.SetAllKeys` "NewEnumerator1") ; Continue from here to do whatever the code should do
    )
    (else
      (`self.SetAllKeys` "NewEnumerator0"))))

(fn `SetAllKeys`
  (params (ActiveKeyState :type "/Game/Blueprints/Keypad/Enum_KeyState Enum" :default "NewEnumerator0"))
  (for _array_element (`self.Keys`)
    (set `/Game/Blueprints/Keypad/KeypadKey_BP.KeyState` ActiveKeyState _array_element)))

(fn `UserConstructionScript`)